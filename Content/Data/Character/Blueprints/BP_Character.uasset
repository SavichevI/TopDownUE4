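; Character Blueprint that handles swapping a picked-up weapon into the player's inventory slots.
; StartSwitchWeapon caches the pickup and shows a switch widget, while EndSitchWeapon clears the cached pickup.
; Number-key actions share one path that asks InventoryComponent to perform the swap, skipping the index matching the last AmmoSlot entry.
; The replaced item spawns as a pickup actor in front of the character, and successful swaps notify the original pickup.
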(event Custom|StartSwitchWeapon
  (params (CatchPickUpWeapon :type Pick%20Up%20Actors%20Object%20Reference))
  (bind _returnvalue (UserInterface|CreateWidget "/Game/Data/FX/Widgets/Inventory/SitchWeaponWidget.SitchWeaponWidget_C"))
  (UserInterface|Viewport|AddtoViewport _returnvalue 0)
  (Variables|Default|SetCatchPickUpWeapon CatchPickUpWeapon))

(event Custom|EndSitchWeapon
  (Variables|Default|SetCatchPickUpWeapon 0))

(event EventTick
  (params (DeltaSeconds :type Float%20%28single-precision%29)))

(event Input|ActionEvents|InputActionActionNum1
  (params (Key :type Key%20Structure :default "None"))
  (bind _catchpickupweapon (Variables|Default|GetCatchPickUpWeapon))
  (:Pressed
    (Variables|Default|SetCurrentIndexToSwitch 0)
    (Utilities|IsValid _catchpickupweapon
      (:Is%20Valid
        (if (not (== (Variables|Default|GetCurrentIndexToSwitch) (- (Utilities|Array|Length (Variables|/Script/TDS.M_InventaryComponent|GetAmmoSlot (Variables|Default|GetInventoryComponent))) 1)))
          (if (not (Utilities|Name|Equal(Name) (.NameItem (Utilities|Struct|BreakWeaponSlot (Variables|/Game/Data/Blueprints/DropActors/PickUpActors.PickUpActors_C|GetWeaponSlot _catchpickupweapon))) "None"))
            (bind (_dropiteminfo _returnvalue) (Class|MInventaryComponent|SwitchWeapontoInventory (Variables|Default|GetInventoryComponent) (Variables|/Game/Data/Blueprints/DropActors/PickUpActors.PickUpActors_C|GetWeaponSlot _catchpickupweapon) (Variables|Default|GetCurrentIndexToSwitch) (Variables|Default|GetCurrentIndexWeapon)))
            (CallFunction|DropItems _dropiteminfo)
            (if _returnvalue
              (Default|PickUpSuccess _catchpickupweapon)))))
      (:Is%20Not%20Valid
        (Development|PrintString "no")))))

(event Input|ActionEvents|InputActionActionNum2
  (params (Key :type Key%20Structure :default "None"))
  (bind _catchpickupweapon (Variables|Default|GetCatchPickUpWeapon))
  (:Pressed
    (Variables|Default|SetCurrentIndexToSwitch 1)
    (Utilities|IsValid _catchpickupweapon
      (:Is%20Valid
        (if (not (== (Variables|Default|GetCurrentIndexToSwitch) (- (Utilities|Array|Length (Variables|/Script/TDS.M_InventaryComponent|GetAmmoSlot (Variables|Default|GetInventoryComponent))) 1)))
          (if (not (Utilities|Name|Equal(Name) (.NameItem (Utilities|Struct|BreakWeaponSlot (Variables|/Game/Data/Blueprints/DropActors/PickUpActors.PickUpActors_C|GetWeaponSlot _catchpickupweapon))) "None"))
            (bind (_dropiteminfo _returnvalue) (Class|MInventaryComponent|SwitchWeapontoInventory (Variables|Default|GetInventoryComponent) (Variables|/Game/Data/Blueprints/DropActors/PickUpActors.PickUpActors_C|GetWeaponSlot _catchpickupweapon) (Variables|Default|GetCurrentIndexToSwitch) (Variables|Default|GetCurrentIndexWeapon)))
            (CallFunction|DropItems _dropiteminfo)
            (if _returnvalue
              (Default|PickUpSuccess _catchpickupweapon)))))
      (:Is%20Not%20Valid
        (Development|PrintString "no")))))

(event Input|ActionEvents|InputActionActionNum3
  (params (Key :type Key%20Structure :default "None"))
  (bind _catchpickupweapon (Variables|Default|GetCatchPickUpWeapon))
  (:Pressed
    (Variables|Default|SetCurrentIndexToSwitch 2)
    (Utilities|IsValid _catchpickupweapon
      (:Is%20Valid
        (if (not (== (Variables|Default|GetCurrentIndexToSwitch) (- (Utilities|Array|Length (Variables|/Script/TDS.M_InventaryComponent|GetAmmoSlot (Variables|Default|GetInventoryComponent))) 1)))
          (if (not (Utilities|Name|Equal(Name) (.NameItem (Utilities|Struct|BreakWeaponSlot (Variables|/Game/Data/Blueprints/DropActors/PickUpActors.PickUpActors_C|GetWeaponSlot _catchpickupweapon))) "None"))
            (bind (_dropiteminfo _returnvalue) (Class|MInventaryComponent|SwitchWeapontoInventory (Variables|Default|GetInventoryComponent) (Variables|/Game/Data/Blueprints/DropActors/PickUpActors.PickUpActors_C|GetWeaponSlot _catchpickupweapon) (Variables|Default|GetCurrentIndexToSwitch) (Variables|Default|GetCurrentIndexWeapon)))
            (CallFunction|DropItems _dropiteminfo)
            (if _returnvalue
              (Default|PickUpSuccess _catchpickupweapon)))))
      (:Is%20Not%20Valid
        (Development|PrintString "no")))))

(event Input|ActionEvents|InputActionActionNum4
  (params (Key :type Key%20Structure :default "None"))
  (bind _catchpickupweapon (Variables|Default|GetCatchPickUpWeapon))
  (:Pressed
    (Variables|Default|SetCurrentIndexToSwitch 3)
    (Utilities|IsValid _catchpickupweapon
      (:Is%20Valid
        (if (not (== (Variables|Default|GetCurrentIndexToSwitch) (- (Utilities|Array|Length (Variables|/Script/TDS.M_InventaryComponent|GetAmmoSlot (Variables|Default|GetInventoryComponent))) 1)))
          (if (not (Utilities|Name|Equal(Name) (.NameItem (Utilities|Struct|BreakWeaponSlot (Variables|/Game/Data/Blueprints/DropActors/PickUpActors.PickUpActors_C|GetWeaponSlot _catchpickupweapon))) "None"))
            (bind (_dropiteminfo _returnvalue) (Class|MInventaryComponent|SwitchWeapontoInventory (Variables|Default|GetInventoryComponent) (Variables|/Game/Data/Blueprints/DropActors/PickUpActors.PickUpActors_C|GetWeaponSlot _catchpickupweapon) (Variables|Default|GetCurrentIndexToSwitch) (Variables|Default|GetCurrentIndexWeapon)))
            (CallFunction|DropItems _dropiteminfo)
            (if _returnvalue
              (Default|PickUpSuccess _catchpickupweapon)))))
      (:Is%20Not%20Valid
        (Development|PrintString "no")))))

(fn ConstructionScript)

(fn DropItems
  (params (Drop%20Item%20Info :type Drop%20Item%20Structure))
  (bind _returnvalue (Game|SpawnActorfromClass "/Game/Data/Blueprints/DropActors/PickUpActors_Weapon.PickUpActors_Weapon_C" (Math|Transform|MakeTransform (+ (Transformation|GetActorLocation) (* (Transformation|GetActorForwardVector) 1e+02))) "Undefined" 0 0))
  (Default|InitActor _returnvalue Drop%20Item%20Info))