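; BP_Computer is a computer prop whose monitor can flicker, with an optional particle effect.
; BeginPlay creates a dynamic material instance on the Monitor mesh and, if WorkingMonitor is set, starts a looping timer that calls Flicker.
; Flicker alternates the screen's "Intencety" parameter between lit and offline values.
; The Construction Script sets particle visibility and also calls Flicker for working monitors, although the dynamic material is only created at BeginPlay.
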(event EventBeginPlay
  (bind _returnvalue (Rendering|Material|CreateDynamicMaterialInstance (Variables|Default|GetMonitor) 3 "/Game/Data/Meshes/Environment/Materials/Light/MI_Light_Monitor.MI_Light_Monitor" "None" :!class /Script/Engine.PrimitiveComponent))
  (Variables|Components|SetMaterialMonitor _returnvalue)
  (if (Variables|Customize|GetWorkingMonitor)
    (Utilities|Time|SetTimerbyFunctionName 0 "Flicker" (Variables|Customize|GetTimer) true)))

(event Collision|EventActorBeginOverlap
  (params (OtherActor :type Actor%20Object%20Reference)))

(event EventTick
  (params (DeltaSeconds :type Float%20%28single-precision%29)))

(fn ConstructionScript
  (if (Variables|Customize|GetWorkingMonitor)
    (CallFunction|Flicker))
  (Rendering|SetVisibility (Variables|Default|GetParticleSystem) (Variables|Customize|GetVisibilityParticle) false))

(fn Flicker
  (if (Variables|Components|GetbVisibilityLight)
    (Rendering|Material|SetScalarParameterValue (Variables|Components|GetMaterialMonitor) "Intencety" (Variables|Customize|GetIntencetyForLight) :!class /Script/Engine.MaterialInstanceDynamic)
    (Variables|Components|SetbVisibilityLight false)
    (else
      (Rendering|Material|SetScalarParameterValue (Variables|Components|GetMaterialMonitor) "Intencety" (Variables|Components|GetIntencetyOffline) :!class /Script/Engine.MaterialInstanceDynamic)
      (Variables|Components|SetbVisibilityLight true))))