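; BP_Door is a double door that swings open when BP_Character enters its trigger box and closes on exit.
; When locked it requires the character's Key, otherwise playing a sound and printing a message; an optional cap is destroyed on opening.
; Looping timers rotate both leaves in mirrored steps with collision off, until yaw reaches its limit.
; The construction script caches closed rotation and collision, and configures sound parameters.
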(event OnComponentBeginOverlap(Box)
  (params (OverlappedComponent :type Primitive%20Component%20Object%20Reference) (OtherActor :type Actor%20Object%20Reference) (OtherComp :type Primitive%20Component%20Object%20Reference) (OtherBodyIndex :type Integer) (bFromSweep :type Boolean) (SweepResult :type Hit%20Result%20Structure%20%28by%20ref%29))
  (bind _asbp_character (Utilities|Casting|CastToBP_Character OtherActor))
  (if (Variables|Customize|GetbBeClose)
    (if (Variables|/Game/Data/Character/Blueprints/BP_Character.BP_Character_C|GetKey _asbp_character)
      (if (Variables|Customize|GetbBeCap) :!label _label
        (Actor|DestroyActor (Variables|Customize|GetCap))
        (Variables|Customize|SetbBeCap false))
      (if (not (Variables|Animation|GetbOpen))
        (Utilities|Time|SetTimerbyFunctionName 0 "FOpenDoor" (Variables|Animation|GetIsTimeAnimationDoor) true)
        (if (Variables|Sound|GetbOnVolume)
          (Audio|Components|Audio|Play (Variables|Default|GetOpenDoor) 0.0)))
      (else
        (Audio|Components|Audio|Play (Variables|Default|GetCue_ClosedDoor) 0.0)
        (Development|PrintString (Variables|Customize|GetIn%20String) true true "(R=1.000000,G=0.000000,B=0.000000,A=1.000000)" 2e+01)))
    (else
      (goto _label))))

(event OnComponentEndOverlap(Box)
  (params (OverlappedComponent :type Primitive%20Component%20Object%20Reference) (OtherActor :type Actor%20Object%20Reference) (OtherComp :type Primitive%20Component%20Object%20Reference) (OtherBodyIndex :type Integer))
  (Utilities|Casting|CastToBP_Character OtherActor)
  (if (Variables|Animation|GetbOpen)
    (Utilities|Time|SetTimerbyFunctionName 0 "FCloseDoor" (Variables|Animation|GetIsTimeAnimationDoor) true)))

(event EventBeginPlay)

(event Collision|EventActorBeginOverlap
  (params (OtherActor :type Actor%20Object%20Reference)))

(event EventTick
  (params (DeltaSeconds :type Float%20%28single-precision%29)))

(fn ConstructionScript
  (bind _opendoor (Variables|Default|GetOpenDoor))
  (bind _door (Variables|Default|GetDoor))
  (Variables|Animation|SetOldRotation (Variables|/Script/Engine.SceneComponent|GetRelativeRotation _door))
  (Variables|Customize|SetIsCollision (Collision|GetCollisionEnabled _door))
  (Effects|Components|ParticleSystem|SetBoolParameter _opendoor "play" (Variables|Sound|GetbOnVolume))
  (Audio|Parameter|SetFloatParameter _opendoor "volume" (Variables|Sound|GetOpenDoorVolume) :!class /Script/Engine.AudioComponent))

(fn FOpenDoor
  (bind _directiondoor (Variables|Animation|GetDirectionDoor))
  (bind _door (Variables|Default|GetDoor))
  (bind _relativerotation (Variables|/Script/Engine.SceneComponent|GetRelativeRotation _door))
  (Collision|SetCollisionEnabled (Variables|Default|GetDoor_2) "NoCollision")
  (Transformation|AddRelativeRotation _door _directiondoor false false)
  (Transformation|AddRelativeRotation (Variables|Default|GetDoor_2) (* _directiondoor -1.0) false false)
  (if (Math|Rotator|Equal(Rotator) (Variables|Animation|GetDirectionDoor) "0,-1.000000, 0" 0.0001)
    (bind _output_get (Variables|Animation|SetIsRotation _relativerotation))
    (if (<= (.yaw _output_get) (.yaw (Variables|Animation|GetHowOpenDoor)))
      (Class|KismetSystemLibrary|PauseTimer 0 "FOpenDoor" :!label _label)
      (Collision|SetCollisionEnabled (Variables|Default|GetDoor) (Variables|Customize|GetIsCollision))
      (Audio|Components|Audio|Stop (Variables|Default|GetOpenDoor))
      (Variables|Animation|SetbOpen true))
    (else
      (bind _output_get_2 (Variables|Animation|SetIsRotation _relativerotation))
      (if (>= (.yaw _output_get_2) (.yaw (Variables|Animation|GetHowOpenDoor)))
        (goto _label)))))

(fn FCloseDoor
  (bind _door (Variables|Default|GetDoor))
  (bind _directiondoor (Variables|Animation|GetDirectionDoor))
  (bind _relativerotation (Variables|/Script/Engine.SceneComponent|GetRelativeRotation _door))
  (Collision|SetCollisionEnabled (Variables|Default|GetDoor_2) "NoCollision")
  (Transformation|AddRelativeRotation (Variables|Default|GetDoor) (* _directiondoor -1.0) false false)
  (Transformation|AddRelativeRotation (Variables|Default|GetDoor_2) _directiondoor false false)
  (if (Math|Rotator|Equal(Rotator) (Variables|Animation|GetDirectionDoor) "0,-1.000000, 0" 0.0001)
    (bind _output_get (Variables|Animation|SetIsRotation _relativerotation))
    (if (>= (.yaw _output_get) (.yaw (Variables|Animation|GetOldRotation)))
      (if (Variables|Sound|GetbOnVolume) :!label _label
        (Audio|Components|Audio|Play (Variables|Default|GetCue_ClosingDoor) 0.0))
      (Class|KismetSystemLibrary|PauseTimer 0 "FCloseDoor")
      (Transformation|SetRelativeRotation (Variables|Default|GetDoor) (Variables|Animation|GetOldRotation) false false)
      (Collision|SetCollisionEnabled (Variables|Default|GetDoor) (Variables|Customize|GetIsCollision))
      (Variables|Animation|SetbOpen false))
    (else
      (bind _output_get_2 (Variables|Animation|SetIsRotation _relativerotation))
      (if (<= (.yaw _output_get_2) (.yaw (Variables|Animation|GetOldRotation)))
        (goto _label)))))