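; BP_Chair is a chair actor with customizable colors and surface normal, built from Seat, Back and Legs components.
; The construction script calls CustomizeColor, which creates a dynamic material instance for slot 0 of each component.
; Seat and Back share a color and normal texture, while Legs get only their own color, all colors using the misspelled "Bace Color" parameter.
; It has no runtime logic, as the event graph holds only disabled stub events.
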(event EventBeginPlay)

(event Collision|EventActorBeginOverlap
  (params (OtherActor :type Actor%20Object%20Reference)))

(event EventTick
  (params (DeltaSeconds :type Float%20%28single-precision%29)))

(fn ConstructionScript
  (CallFunction|CustomizeColor))

(fn CustomizeColor
  (Utilities|FlowControl|Sequence
    (:then_0
      (bind _returnvalue (Rendering|Material|CreateDynamicMaterialInstance (Variables|Default|GetSeat) 0 0 "None" :!class /Script/Engine.PrimitiveComponent))
      (Rendering|Material|SetVectorParameterValue _returnvalue "Bace Color" (Variables|Default|GetColorForChair) :!class /Script/Engine.MaterialInstanceDynamic :!label _label)
      (Rendering|Material|SetTextureParameterValue _returnvalue "Normal" (Variables|Default|GetNormalForChair)))
    (:then_1
      (bind _returnvalue_2 (Rendering|Material|CreateDynamicMaterialInstance (Variables|Default|GetBack) 0 0 "None" :!class /Script/Engine.PrimitiveComponent))
      (goto _label))
    (:then_2
      (bind _returnvalue_3 (Rendering|Material|CreateDynamicMaterialInstance (Variables|Default|GetLegs) 0 0 "None" :!class /Script/Engine.PrimitiveComponent))
      (Rendering|Material|SetVectorParameterValue _returnvalue_3 "Bace Color" (Variables|Default|GetColorForLegs) :!class /Script/Engine.MaterialInstanceDynamic))))