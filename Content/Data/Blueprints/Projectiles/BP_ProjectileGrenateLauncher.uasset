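; Grenade launcher projectile that deals area damage to BP_Enemy actors when destroyed.
; On Destroyed, a sphere trace for pawns lowers CurrentHP on newly hit enemies.
; Each such hit triggers a second trace using the SphereOfDistanceDamage radius for another, larger HP deduction, printing the result.
; Separate arrays prevent repeat damage within each trace tier; the SphereDemegeMax helper is never called here.
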(event EventBeginPlay)

(event Collision|EventActorBeginOverlap
  (params (OtherActor :type Actor%20Object%20Reference)))

(event EventTick
  (params (DeltaSeconds :type Float%20%28single-precision%29)))

(event EventDestroyed
  (bind _returnvalue (Transformation|GetActorLocation))
  (bind _returnvalue_2 (Transformation|GetActorLocation))
  (bind _outhits (Collision|MultiSphereTraceForObjects _returnvalue_2 (+ _returnvalue_2 "0, 0,1.000000") (Variables|Default|GetRadius) (Utilities|Array|MakeArray "ObjectTypeQuery3") false 0 "None"))
  (for _array_element _outhits
    (Variables|Default|SetHit%20Actor (.HitActor (Collision|BreakHitResult _array_element)))
    (if (not (Utilities|Array|ContainsItem (Variables|Default|GetHit%20Actor%20Max%20Demege) (Variables|Default|GetHit%20Actor)))
      (bind _returnvalue_3 (Utilities|Array|Add (Variables|Default|GetHit%20Actor%20Max%20Demege) (Variables|Default|GetHit%20Actor)))
      (bind _asbp_enemy (Utilities|Casting|CastToBP_Enemy (Utilities|Array|Get(acopy) (Variables|Default|GetHit%20Actor%20Max%20Demege) _returnvalue_3)))
      (Variables|/Game/Data/Blueprints/Enemy/BP_Enemy.BP_Enemy_C|SetCurrentHP _asbp_enemy (- (Variables|/Game/Data/Blueprints/Enemy/BP_Enemy.BP_Enemy_C|GetCurrentHP _asbp_enemy) 5e+01))
      (bind _outhits_2 (Collision|MultiSphereTraceForObjects _returnvalue (+ _returnvalue "0, 0,1.000000") (Variables|/Script/Engine.SphereComponent|GetSphereRadius (Variables|Default|GetSphereOfDistanceDamage)) (Utilities|Array|MakeArray "ObjectTypeQuery3") false 0 "None"))
      (for _array_element_2 _outhits_2
        (Variables|Default|SetHit%20Actor (.HitActor (Collision|BreakHitResult _array_element_2)))
        (if (not (Utilities|Array|ContainsItem (Variables|Default|GetHit%20Actor%20Min%20Demege) (Variables|Default|GetHit%20Actor)))
          (bind _returnvalue_4 (Utilities|Array|Add (Variables|Default|GetHit%20Actor%20Min%20Demege) (Variables|Default|GetHit%20Actor)))
          (bind _asbp_enemy_2 (Utilities|Casting|CastToBP_Enemy (Utilities|Array|Get(acopy) (Variables|Default|GetHit%20Actor%20Min%20Demege) _returnvalue_4)))
          (bind _output_get (Variables|/Game/Data/Blueprints/Enemy/BP_Enemy.BP_Enemy_C|SetCurrentHP _asbp_enemy_2 (- (Variables|/Game/Data/Blueprints/Enemy/BP_Enemy.BP_Enemy_C|GetCurrentHP _asbp_enemy_2) 2e+02)))
          (Development|PrintString (Utilities|String|ToString(Float) _output_get)))))))

(fn ConstructionScript)

(fn SphereDemegeMax
  (params (RadiusSphere :type Float%20%28single-precision%29))
  (bind _returnvalue (Transformation|GetActorLocation))
  (bind _outhits (Collision|MultiSphereTraceForObjects _returnvalue (+ _returnvalue "0, 0,1.000000") RadiusSphere (Utilities|Array|MakeArray "ObjectTypeQuery3") false 0 "None"))
  (for _array_element _outhits
    (Variables|Default|SetHit%20Actor (.HitActor (Collision|BreakHitResult _array_element)))
    (if (not (Utilities|Array|ContainsItem (Variables|Default|GetHit%20Actor%20Max%20Demege) (Variables|Default|GetHit%20Actor)))
      (bind _returnvalue_2 (Utilities|Array|Add (Variables|Default|GetHit%20Actor%20Max%20Demege) (Variables|Default|GetHit%20Actor)))
      (return 0 (Utilities|Array|Get(acopy) (Variables|Default|GetHit%20Actor%20Max%20Demege) _returnvalue_2)))))