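; Ammo pickup actor that refills a character's ammo for its weapon type, built as a child of a base pickup class.
; On character overlap it asks the inventory component whether that weapon type can take ammo.
; If so, it adds its count to the matching ammo slot and signals a successful pickup.
; Construction and drop-item initialization only call the parent implementations.
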(event EventBeginPlay
  (|CallParentFunction) ; This node is disabled and will not be called.\nDrag off pins to build functionality.
)

(event Collision|EventActorBeginOverlap
  (params (OtherActor :type Actor%20Object%20Reference))
  (|CallParentFunction OtherActor) ; This node is disabled and will not be called.\nDrag off pins to build functionality.
)

(event EventTick
  (params (DeltaSeconds :type Float%20%28single-precision%29))
  (|CallParentFunction DeltaSeconds) ; This node is disabled and will not be called.\nDrag off pins to build functionality.
)

(event EventOverlapCharacter
  (params (InventoryComponent :type M%20Inventary%20Component%20Object%20Reference))
  (bind _weapontype (Variables|Default|GetWeaponType))
  (|CallParentFunction InventoryComponent)
  (bind _returnvalue (Class|MInventaryComponent|CheckCanTakeAmmo InventoryComponent _weapontype))
  (if _returnvalue
    (Class|MInventaryComponent|AmmoSlotChangeValue InventoryComponent _weapontype (Variables|Default|GetCout))
    (CallFunction|PickUpSuccess)))

(fn ConstructionScript
  (|CallParentFunction))

(fn InitActor
  (params (DropItemInfo :type Drop%20Item%20Structure))
  (|CallParentFunction DropItemInfo))