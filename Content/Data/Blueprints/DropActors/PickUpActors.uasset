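; Base pickup actor for dropped items that characters collect by overlapping it.
; Its Sphere overlap casts the other actor to BP_Character and passes that character's InventoryComponent to OverlapCharacter, an empty event here that serves as a hook.
; InitActor sets up the static mesh from the drop item info, or destroys the mesh component and prints a warning if no weapon mesh is valid.
; PickUpSuccess destroys the actor.
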(event OnComponentBeginOverlap(Sphere)
  (params (OverlappedComponent :type Primitive%20Component%20Object%20Reference) (OtherActor :type Actor%20Object%20Reference) (OtherComp :type Primitive%20Component%20Object%20Reference) (OtherBodyIndex :type Integer) (bFromSweep :type Boolean) (SweepResult :type Hit%20Result%20Structure%20%28by%20ref%29))
  (bind _asbp_character (Utilities|Casting|CastToBP_Character OtherActor))
  (CallFunction|OverlapCharacter (Variables|/Script/TDS.TDSCharacter|GetInventoryComponent _asbp_character)))

(event Custom|OverlapCharacter
  (params (InventoryComponent :type M%20Inventary%20Component%20Object%20Reference)))

(event EventBeginPlay)

(event Collision|EventActorBeginOverlap
  (params (OtherActor :type Actor%20Object%20Reference)))

(event EventTick
  (params (DeltaSeconds :type Float%20%28single-precision%29)))

(fn ConstructionScript)

(fn PickUpSuccess
  (Actor|DestroyActor))

(fn InitActor
  (params (DropItemInfo :type Drop%20Item%20Structure))
  (bind _staticmesh (Variables|Default|GetStaticMesh))
  (Utilities|IsValid (.WeaponStaticMesh (Utilities|Struct|BreakDropItem DropItemInfo))
    (:Is%20Valid
      (Components|StaticMesh|SetStaticMesh _staticmesh 0))
    (:Is%20Not%20Valid
      (Components|DestroyComponent _staticmesh)
      (Development|PrintString "Not Static Mesh" true true "(R=0.718750,G=0.000000,B=0.041368,A=1.000000)" 0.0))))