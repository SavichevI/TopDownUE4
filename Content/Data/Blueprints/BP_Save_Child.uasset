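; BP_Save_Child is a trigger actor that grants the player a key when the character enters its box.
; On Box overlap, it casts the other actor to BP_Character, sets that character's Key flag and prints a green on-screen message about killing monsters.
; The construction script only calls its parent, and the stubbed BeginPlay, Tick and actor overlap events are disabled.
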(event OnComponentBeginOverlap(Box)
  (params (OverlappedComponent :type Primitive%20Component%20Object%20Reference) (OtherActor :type Actor%20Object%20Reference) (OtherComp :type Primitive%20Component%20Object%20Reference) (OtherBodyIndex :type Integer) (bFromSweep :type Boolean) (SweepResult :type Hit%20Result%20Structure%20%28by%20ref%29))
  (bind _asbp_character (Utilities|Casting|CastToBP_Character OtherActor))
  (Variables|/Game/Data/Character/Blueprints/BP_Character.BP_Character_C|SetKey _asbp_character true)
  (Development|PrintString "Cool. You kill monstar. Mach monstors." true true "(R=0.000000,G=1.000000,B=0.000000,A=1.000000)"))

(event EventBeginPlay
  (|CallParentFunction) ; This node is disabled and will not be called.\nDrag off pins to build functionality.
)

(event Collision|EventActorBeginOverlap
  (params (OtherActor :type Actor%20Object%20Reference))
  (|CallParentFunction OtherActor) ; This node is disabled and will not be called.\nDrag off pins to build functionality.
)

(event EventTick
  (params (DeltaSeconds :type Float%20%28single-precision%29))
  (|CallParentFunction DeltaSeconds) ; This node is disabled and will not be called.\nDrag off pins to build functionality.
)

(fn ConstructionScript
  (|CallParentFunction))