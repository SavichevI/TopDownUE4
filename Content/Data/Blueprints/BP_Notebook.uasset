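; Configurable notebook prop that can appear closed, broken or with a blinking screen light, with optional electricity particles and sound.
; The construction script recolors body and label via dynamic material instances, poses the monitor, repositions particles for closed or broken states, and sets particle visibility and sound parameters.
; BeginPlay starts the sound if particles are visible and, if WorkingMonitore is set, loops a timer on Working to toggle screen intensity.
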(event EventBeginPlay
  (if (Variables|Customize|GetbVisibilityParticle)
    (Audio|Components|Audio|Play (Variables|Default|GetCue_Electricity) 0.0))
  (if (Variables|Customize|GetbWorkingMonitore)
    (Utilities|Time|SetTimerbyFunctionName 0 "Working" (Variables|Customize|GetTiming) true)))

(event Collision|EventActorBeginOverlap
  (params (OtherActor :type Actor%20Object%20Reference)))

(event EventTick
  (params (DeltaSeconds :type Float%20%28single-precision%29)))

(fn ConstructionScript
  (bind _cue_electricity (Variables|Default|GetCue_Electricity))
  (CallFunction|CustomizeColor)
  (if (Variables|Customize|GetbClosedNotebook)
    (Transformation|SetRelativeTransform (Variables|Default|GetMonitore) (Variables|Components|GetClosedNoebook) false false)
    (Transformation|SetRelativeLocation (Variables|Default|GetParticleSystem) (Variables|Components|GetLocationForParticle) false false :!label _label)
    (elif (Variables|Customize|GetbBrokenNotebook)
      (Transformation|SetRelativeTransform (Variables|Default|GetMonitore) (Variables|Customize|GetBrokenNotebook) false false)
      (goto _label)
      (elif (Variables|Customize|GetbWorkingMonitore)
        (CallFunction|Working))))
  (Rendering|SetVisibility (Variables|Default|GetParticleSystem) (Variables|Customize|GetbVisibilityParticle) false)
  (Effects|Components|ParticleSystem|SetBoolParameter _cue_electricity "play" (Variables|Sound|GetbOnVolume))
  (Audio|Parameter|SetFloatParameter _cue_electricity "volume" (Variables|Sound|GetElectricityVolume) :!class /Script/Engine.AudioComponent))

(fn Working
  (if (Variables|Components|GetbOffWork)
    (bind _returnvalue (Rendering|Material|CreateDynamicMaterialInstance (Variables|Default|GetMonitore) 4 "/Game/Data/Meshes/Environment/Materials/Light/MI_Light_Monitor.MI_Light_Monitor" "None" :!class /Script/Engine.PrimitiveComponent))
    (Rendering|Material|SetScalarParameterValue _returnvalue "Intencety" (Variables|Customize|GetIntencety) :!class /Script/Engine.MaterialInstanceDynamic)
    (Variables|Components|SetbOffWork false)
    (else
      (bind _returnvalue_2 (Rendering|Material|CreateDynamicMaterialInstance (Variables|Default|GetMonitore) 4 "/Game/Data/Meshes/Environment/Materials/Light/MI_Light_Monitor.MI_Light_Monitor" "None" :!class /Script/Engine.PrimitiveComponent))
      (Rendering|Material|SetScalarParameterValue _returnvalue_2 "Intencety" 0.0 :!class /Script/Engine.MaterialInstanceDynamic)
      (Variables|Components|SetbOffWork true))))

(fn CustomizeColor
  (Utilities|FlowControl|Sequence
    (:then_0
      (bind _returnvalue (Rendering|Material|CreateDynamicMaterialInstance (Variables|Default|GetMonitore) 0 "/Game/Data/Meshes/Environment/Materials/Computer/MI_Computer.MI_Computer" "None" :!class /Script/Engine.PrimitiveComponent))
      (Rendering|Material|SetVectorParameterValue _returnvalue "Bace Color" (Variables|Customize|GetBaceColor) :!class /Script/Engine.MaterialInstanceDynamic :!label _label))
    (:then_1
      (bind _returnvalue_2 (Rendering|Material|CreateDynamicMaterialInstance (Variables|Default|GetMonitore) 3 "/Game/Data/Meshes/Environment/Materials/Computer/MI_Computer.MI_Computer" "None" :!class /Script/Engine.PrimitiveComponent))
      (goto _label))
    (:then_2
      (bind _returnvalue_3 (Rendering|Material|CreateDynamicMaterialInstance (Variables|Default|GetNoteBook) 2 "/Game/Data/Meshes/Environment/Materials/Computer/MI_Computer.MI_Computer" "None" :!class /Script/Engine.PrimitiveComponent))
      (goto _label))
    (:then_3
      (bind _returnvalue_4 (Rendering|Material|CreateDynamicMaterialInstance (Variables|Default|GetNoteBook) 3 "/Game/Data/Meshes/Environment/Materials/Computer/MI_Computer.MI_Computer" "None" :!class /Script/Engine.PrimitiveComponent))
      (goto _label))
    (:then_4
      (bind _returnvalue_5 (Rendering|Material|CreateDynamicMaterialInstance (Variables|Default|GetNoteBook) 6 "/Game/Data/Meshes/Environment/Materials/Computer/MI_Computer.MI_Computer" "None" :!class /Script/Engine.PrimitiveComponent))
      (goto _label))
    (:then_5
      (bind _returnvalue_6 (Rendering|Material|CreateDynamicMaterialInstance (Variables|Default|GetMonitore) 2 "/Game/Data/Meshes/Environment/Materials/Computer/MI_Computer.MI_Computer" "None" :!class /Script/Engine.PrimitiveComponent))
      (Rendering|Material|SetVectorParameterValue _returnvalue_6 "Bace Color" (Variables|Customize|GetColorForLabel) :!class /Script/Engine.MaterialInstanceDynamic))))