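; BP_Sink is a sink prop that can be configured as broken, with visible water and particles, or intact, with optional running-water sound.
; The construction script ties water and particle visibility to Broken, applies the water transform, and passes play and volume parameters to both audio cues.
; BeginPlay starts the broken-faucet cue when Broken is set, otherwise the running-water cue if SoundRunningWater is enabled.
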(event EventBeginPlay
  (if (Variables|Default|GetbBroken)
    (Audio|Components|Audio|Play (Variables|Default|GetCue_BrokenFaucet) 0.0)
    (elif (Variables|Default|GetbSoundRunningWater)
      (Audio|Components|Audio|Play (Variables|Default|GetCue_WaterRunning) 0.0))))

(event Collision|EventActorBeginOverlap
  (params (OtherActor :type Actor%20Object%20Reference)))

(event EventTick
  (params (DeltaSeconds :type Float%20%28single-precision%29)))

(fn ConstructionScript
  (bind _bbroken (Variables|Default|GetbBroken))
  (bind _cue_waterrunning (Variables|Default|GetCue_WaterRunning))
  (Rendering|SetVisibility (Variables|Default|GetParticleSystem) _bbroken false)
  (Rendering|SetVisibility (Variables|Default|GetWater) _bbroken false)
  (Transformation|SetRelativeTransform (Variables|Default|GetWater) (Variables|Default|GetTransformForWater) false false)
  (Effects|Components|ParticleSystem|SetBoolParameter _cue_waterrunning "play" (Variables|Sound|GetbOn%20Volume))
  (Audio|Parameter|SetFloatParameter _cue_waterrunning "volume" (Variables|Sound|GetWaterVolume) :!class /Script/Engine.AudioComponent))