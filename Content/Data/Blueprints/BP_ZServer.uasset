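; BP_ZServer is an actor that plays a server sound while a BP_Character is inside its box trigger.
; The construction script assigns Cue_Server to the CueServer audio component and passes OnVolum and SoundVolume into its "play" and "volume" sound parameters.
; Box overlap begin starts the audio from the beginning, and overlap end stops it.
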(event OnComponentBeginOverlap(Box)
  (params (OverlappedComponent :type Primitive%20Component%20Object%20Reference) (OtherActor :type Actor%20Object%20Reference) (OtherComp :type Primitive%20Component%20Object%20Reference) (OtherBodyIndex :type Integer) (bFromSweep :type Boolean) (SweepResult :type Hit%20Result%20Structure%20%28by%20ref%29))
  (Utilities|Casting|CastToBP_Character OtherActor)
  (Audio|Components|Audio|Play (Variables|Default|GetCue_Server) 0.0))

(event OnComponentEndOverlap(Box)
  (params (OverlappedComponent :type Primitive%20Component%20Object%20Reference) (OtherActor :type Actor%20Object%20Reference) (OtherComp :type Primitive%20Component%20Object%20Reference) (OtherBodyIndex :type Integer))
  (Utilities|Casting|CastToBP_Character OtherActor)
  (Audio|Components|Audio|Stop (Variables|Default|GetCue_Server)))

(event EventBeginPlay)

(event Collision|EventActorBeginOverlap
  (params (OtherActor :type Actor%20Object%20Reference)))

(event EventTick
  (params (DeltaSeconds :type Float%20%28single-precision%29)))

(fn ConstructionScript
  (bind _cue_server (Variables|Default|GetCue_Server))
  (Audio|Components|Audio|SetSound _cue_server "/Game/Data/Sounds/Enviroment/Cue_Server.Cue_Server")
  (Effects|Components|ParticleSystem|SetBoolParameter _cue_server "play" (Variables|Sound|GetbOnVolum))
  (Audio|Parameter|SetFloatParameter _cue_server "volume" (Variables|Sound|GetSoundVolume) :!class /Script/Engine.AudioComponent))